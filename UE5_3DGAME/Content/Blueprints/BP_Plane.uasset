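; BP_Plane is a plane actor that flies forward continuously and rolls with player input.
; Tick moves the actor along its forward vector at MoveSpeed, scaled by delta time, without sweep collision checks.
; The Turn input axis adds local roll to the Body component at RotateSpeed, also scaled by frame time.
; BeginPlay, ActorBeginOverlap and the construction script are empty.
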(event EventBeginPlay)

(event Collision|EventActorBeginOverlap
  (params (OtherActor :type Actor%20Object%20Reference)))

(event EventTick
  (params (DeltaSeconds :type Float%20%28single-precision%29))
  (Transformation|SetActorLocation (+ (Transformation|GetActorLocation) (* (Transformation|GetActorForwardVector) (* DeltaSeconds (Variables|Default|GetMoveSpeed)))) false false))

(event Input|AxisEvents|InputAxisTurn
  (params (AxisValue :type Float%20%28single-precision%29))
  (if (!= AxisValue 0.0)
    (Transformation|AddLocalRotation (Variables|Default|GetBody) (Math|Rotator|MakeRotator (* AxisValue (* (Variables|Default|GetRotateSpeed) (Utilities|Time|GetWorldDeltaSeconds))) 0.0 0.0) false false)))

(fn ConstructionScript)